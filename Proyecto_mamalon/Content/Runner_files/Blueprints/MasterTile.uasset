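; Base track tile for a three-lane endless runner that populates itself and keeps the run going.
; On BeginPlay it randomly spawns a pipe, box or coin in one of three lanes, or leaves the tile empty.
; When the player overlaps its Box, it asks the GameMode for a new tile, adds multiplier-scaled points and raises walk speed within clamped limits.
; The tile then destroys itself after a short delay.
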(event OnComponentBeginOverlap(Box)
  (params (OverlappedComponent :type Primitive%20Component%20Object%20Reference) (OtherActor :type Actor%20Object%20Reference) (OtherComp :type Primitive%20Component%20Object%20Reference) (OtherBodyIndex :type Integer) (bFromSweep :type Boolean) (SweepResult :type Hit%20Result%20Structure%20%28by%20ref%29))
  (Utilities|Casting|CastToThirdPersonCharacter OtherActor)
  (bind _asthird_person_game_mode (Utilities|Casting|CastToThirdPersonGameMode (Game|GetGameMode)))
  (Default|SpawnTile _asthird_person_game_mode)
  (bind _asthird_person_game_mode_2 (Utilities|Casting|CastToThirdPersonGameMode (Game|GetGameMode)))
  (bind _output_get (Variables|/Game/ThirdPersonBP/Blueprints/ThirdPersonGameMode.ThirdPersonGameMode_C|SetCurrentPoints _asthird_person_game_mode_2 (+ (* 15 (Variables|/Game/ThirdPersonBP/Blueprints/ThirdPersonGameMode.ThirdPersonGameMode_C|GetPointsMultiplier _asthird_person_game_mode_2)) (Variables|/Game/ThirdPersonBP/Blueprints/ThirdPersonGameMode.ThirdPersonGameMode_C|GetCurrentPoints _asthird_person_game_mode_2))))
  (Development|PrintString (Utilities|String|ToString(Integer) _output_get))
  (bind _asthird_person_character (Utilities|Casting|CastToThirdPersonCharacter (Game|GetPlayerCharacter 0)))
  (Variables|/Script/Engine.CharacterMovementComponent|SetMaxWalkSpeed (Variables|/Script/Engine.Character|GetCharacterMovement _asthird_person_character) (Math|Float|Clamp(Float) (* (Variables|/Script/Engine.CharacterMovementComponent|GetMaxWalkSpeed (Variables|/Script/Engine.Character|GetCharacterMovement _asthird_person_character)) 1.03) 8e+02 1.6e+03))
  (Utilities|FlowControl|Delay 0.5)
  (Actor|DestroyActor))

(event EventBeginPlay
  (CallFunction|SpawnObstacles))

(event Collision|EventActorBeginOverlap
  (params (OtherActor :type Actor%20Object%20Reference)))

(event EventTick
  (params (DeltaSeconds :type Float%20%28single-precision%29)))

(fn ConstructionScript)

(fn SpawnObstacles
  (switch int (Math|Random|RandomIntegerinRange 0 9)
    (:1
      ;[1 1 1] Spawn Pipe
      (Game|SpawnActorfromClass "/Game/Runner_files/Blueprints/Obstacle_pipe.Obstacle_pipe_C" (Math|Conversions|ToTransform(Vector) (.location (Transformation|GetWorldTransform (Variables|Default|GetLane0)))) "Undefined" 0 0))
    (:2
      (Game|SpawnActorfromClass "/Game/Runner_files/Blueprints/Obstacle_pipe.Obstacle_pipe_C" (Math|Conversions|ToTransform(Vector) (.location (Transformation|GetWorldTransform (Variables|Default|GetLane1)))) "Undefined" 0 0))
    (:3
      (Game|SpawnActorfromClass "/Game/Runner_files/Blueprints/Obstacle_pipe.Obstacle_pipe_C" (Math|Conversions|ToTransform(Vector) (.location (Transformation|GetWorldTransform (Variables|Default|GetLane2)))) "Undefined" 0 0))
    (:4
      ;[1 1 1] Spawn Box
      (Game|SpawnActorfromClass "/Game/Runner_files/Blueprints/Obstacle_box.Obstacle_box_C" (Math|Conversions|ToTransform(Vector) (.location (Transformation|GetWorldTransform (Variables|Default|GetLane0)))) "Undefined" 0 0))
    (:5
      (Game|SpawnActorfromClass "/Game/Runner_files/Blueprints/Obstacle_box.Obstacle_box_C" (Math|Conversions|ToTransform(Vector) (.location (Transformation|GetWorldTransform (Variables|Default|GetLane1)))) "Undefined" 0 0))
    (:6
      (Game|SpawnActorfromClass "/Game/Runner_files/Blueprints/Obstacle_box.Obstacle_box_C" (Math|Conversions|ToTransform(Vector) (.location (Transformation|GetWorldTransform (Variables|Default|GetLane2)))) "Undefined" 0 0))
    (:7
      ;[1 1 1] Spawn Coin
      (Game|SpawnActorfromClass "/Game/Runner_files/Blueprints/Coin_Pickup.Coin_Pickup_C" (Math|Conversions|ToTransform(Vector) (.location (Transformation|GetWorldTransform (Variables|Default|GetLane0)))) "Undefined" 0 0))
    (:8
      (Game|SpawnActorfromClass "/Game/Runner_files/Blueprints/Coin_Pickup.Coin_Pickup_C" (Math|Conversions|ToTransform(Vector) (.location (Transformation|GetWorldTransform (Variables|Default|GetLane1)))) "Undefined" 0 0))
    (:9
      (Game|SpawnActorfromClass "/Game/Runner_files/Blueprints/Coin_Pickup.Coin_Pickup_C" (Math|Conversions|ToTransform(Vector) (.location (Transformation|GetWorldTransform (Variables|Default|GetLane2)))) "Undefined" 0 0))))